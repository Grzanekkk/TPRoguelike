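; Treasure chest interactable that opens only for an instigator holding a required key card gameplay tag.
; Interact checks the instigator's SActionComponent active tags, printing a message naming the missing tag on failure.
; On success a FlipFlop alternates between calling the parent Interact while a timeline rotates the lid open, and reversing that timeline to close it.
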(event EventBeginPlay)

(event Collision|EventActorBeginOverlap
  (params (OtherActor :type Actor%20Object%20Reference)))

(event EventTick
  (params (DeltaSeconds :type Float%20%28single-precision%29)))

(event EventInteract
  (params (Instigator :type Pawn%20Object%20Reference))
  (bind _requiredkeycardtag (Variables|Default|GetRequiredKeyCardTag))
  (if (GameplayTags|HasTag (Variables|/Script/TPRoguelike.SActionComponent|GetActiveGameplayTags (Actor|GetComponentbyClass Instigator "/Script/TPRoguelike.SActionComponent")) _requiredkeycardtag)
    (Utilities|FlowControl|FlipFlop
      (:A
        (|CallParentFunction Instigator)
        (bind _lidrotation (Timeline|AnimateLid Play)
          (:Update
            (Transformation|SetRelativeRotation (Variables|Default|GetLidMesh) (Math|Rotator|MakeRotator 0.0 _lidrotation 0.0) false false))))
      (:B
        (Timeline|AnimateLid Reverse)))
    (else
      (Development|PrintText (Utilities|Text|FormatText "You need: {Kaycard} to open this chest" (GameplayTags|GetTagName _requiredkeycardtag)) true true "(R=1.000000,G=0.467914,B=0.141020,A=1.000000)"))))

(fn ConstructionScript)